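; BP_BetrayalGameState is the game state Blueprint that handles presentation when the match changes stage.
; Exploring starts ambient music and shows a timed, animated game-start widget.
; Haunting swaps the music for the haunting melody, plays a cutscene sequence, unlocks player 0's journal and shows a timed haunt-start widget.
; The Lobby and Finishing stage events are empty.
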(event EventBeginPlay)

(event EventTick
  (params (DeltaSeconds :type Float%20%28single-precision%29)))

(event EventOnHauntingStageStart
  ;[1 1 1] Stage Events
  (Audio|Components|Audio|Stop (Variables|Default|GetAmbient%20music%20))
  (bind _returnvalue (Audio|SpawnSound2D "/Game/Audio/Music/Haunting_Melody_Cue.Haunting_Melody_Cue" 1.0 1.0 0.0 0))
  (Variables|Default|SetAmbient%20music%20 _returnvalue)
  ;[1 1 1] Comment
  (bind _returnvalue_2 (Sequencer|Player|CreateLevelSequencePlayer "/Game/Cutscenes/HauntedMelodyCutscene.HauntedMelodyCutscene"))
  (Sequencer|Player|Play _returnvalue_2 :!class /Script/MovieScene.MovieSceneSequencePlayer)
  (bind _asbp_player_character (Utilities|Casting|CastToBP_PlayerCharacter (Game|Player|GetPlayerPawn 0)))
  (Variables|/Game/Blueprints/BP_PlayerCharacter.BP_PlayerCharacter_C|SetJournalUnlocked _asbp_player_character true)
  (bind _returnvalue_3 (UserInterface|CreateWidget "/Game/UI/Widgets/WB_HauntStart.WB_HauntStart_C" (Game|GetPlayerController 0)))
  (UserInterface|Viewport|AddtoViewport _returnvalue_3 0)
  (UserInterface|Animation|PlayAnimation _returnvalue_3 (Variables|/Game/UI/Widgets/WB_HauntStart.WB_HauntStart_C|GetUI_ANI_HauntStart_1 _returnvalue_3) 0.0 1 "Forward" 1.0 false)
  (Utilities|FlowControl|Delay 8.0)
  (Widget|RemovefromParent _returnvalue_3))

(event EventOnFinishingStageStart
  ;[1 1 1] Stage Events
)

(event EventOnLobbyStageStart
  ;[1 1 1] Stage Events
)

(event EventOnExploringStageStart
  ;[1 1 1] Stage Events
  (bind _returnvalue (Audio|SpawnSound2D "/Game/Audio/Music/Ambient_Music_Cue.Ambient_Music_Cue" 1.0 1.0 0.0 0))
  (Variables|Default|SetAmbient%20music%20 _returnvalue)
  ;[1 1 1] Start Widget
  (Utilities|FlowControl|Delay 1.0)
  (bind _returnvalue_2 (UserInterface|CreateWidget "/Game/UI/Widgets/WB_GameStart.WB_GameStart_C" (Game|GetPlayerController 0)))
  (UserInterface|Viewport|AddtoViewport _returnvalue_2 0)
  (UserInterface|Animation|PlayAnimation _returnvalue_2 (Variables|/Game/UI/Widgets/WB_GameStart.WB_GameStart_C|GetUI_ANI_GameStart _returnvalue_2) 0.0 1 "Forward" 1.0 false)
  (Utilities|FlowControl|Delay 4.1)
  (Widget|RemovefromParent _returnvalue_2))

(fn ConstructionScript)