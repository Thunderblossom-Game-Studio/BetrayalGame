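; Player controller for a betrayal game that owns the local player's HUD, interaction prompt, objective journal and tutorial widget.
; On initialization it caches character and player state references, registers itself on the character and spawns the HUD.
; Events forward health, inventory, portrait and mic changes to the HUD, while input toggles the unlockable journal and opens the tutorial.
; Flashlight and stamina HUD updates are not yet hooked up.
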(event Custom|Show%20HUD
  ;[1 1 1] Spawning the HUD and Interaction Widget
  (Utilities|FlowControl|Sequence
    (:then_0
      (bind _returnvalue (UserInterface|CreateWidget "/Game/UI/Widgets/WB_HUD.WB_HUD_C"))
      (bind _output_get (Variables|Default|SetPlayerHUD _returnvalue))
      (UserInterface|Viewport|AddtoViewport _output_get 0))
    (:then_1
      (bind _returnvalue_2 (UserInterface|CreateWidget "/Game/UI/Widgets/WB_InteractText.WB_InteractText_C"))
      (bind _output_get_2 (Variables|Default|SetInteractionWidget _returnvalue_2))
      (UserInterface|Viewport|AddtoViewport _output_get_2 0))))

(event Custom|Set%20BP%20References
  (params (Character%20Reference :type Player%20Character%20Object%20Reference) (Player%20State%20References :type Betrayal%20Player%20State%20Object%20Reference))
  ;[1 1 1] Setting up the character and player state references
  (bind _asbp_player_character (Utilities|Casting|CastToBP_PlayerCharacter Character%20Reference))
  (Variables|Default|SetCharacterBP _asbp_player_character)
  (bind _asbp_betrayal_player_state (Utilities|Casting|CastToBP_BetrayalPlayerState Player%20State%20References))
  (Variables|Default|SetPlayerStateBP _asbp_betrayal_player_state))

(event Custom|Destroy%20HUD
  ;[1 1 1] Destroying HUD
  (Utilities|FlowControl|Sequence
    (:then_0
      (Widget|RemovefromParent (Variables|Default|GetPlayerHUD)))
    (:then_1
      (Widget|RemovefromParent (Variables|Default|GetInteractionWidget))))
  (Utilities|Platform|CollectGarbage))

(event Custom|Tooltip%20Event%20Widget
  (params (Is%20In%20Focus :type Boolean))
  (bind _interactionwidget (Variables|Default|GetInteractionWidget))
  ;[1 1 1] Tooltip toggle event
  (if Is%20In%20Focus
    (Widget|SetVisibility _interactionwidget "Visible")
    (else
      (Widget|SetVisibility _interactionwidget "Hidden"))))

(event Custom|Update%20Inventory
  (params (Slot :type Inventory%20Slot%20Structure))
  ;[1 1 1] Update Inventory
  (Default|UpdateInventorySlots (Variables|Default|GetPlayerHUD) Slot))

(event Custom|Update%20Player%20Health
  (params (Current%20Health :type Float%20%28double-precision%29) (Max%20Health :type Float%20%28double-precision%29))
  ;[1 1 1] Update Player Health
  (Default|UpdateHealth (Variables|Default|GetPlayerHUD) Current%20Health Max%20Health))

(event Custom|Item%20Equiped
  (params (Slot%20ID :type Inventory%20Slot%20Structure))
  ;[1 1 1] Item Highlight Updates
  (Default|UpdateInventoryHighlight (Variables|Default|GetPlayerHUD) Slot%20ID))

(event Custom|Update%20Picture
  (params (Is%20Traitor :type Boolean))
  ;[1 1 1] Dont work Dont Think.
  (Default|UpdatePlayerPicture (Variables|Default|GetPlayerHUD) Is%20Traitor))

(event Custom|Update%20Mic%20Icon
  (params (Mic%20Muted :type Boolean) (Mic%20Active :type Boolean))
  ;[1 1 1] Update the Microphone icon on the HUD
  (Default|UpdateMicIcon (Variables|Default|GetPlayerHUD) Mic%20Muted Mic%20Active))

(event Custom|Update%20Journal
  (params (New%20State :type Boolean))
  ;[1 1 1] Update Journal
  (Variables|Default|SetJournalUnlocked New%20State))

(event Custom|Set%20Controller%20On%20Character
  ;[1 1 1] Setting up the player controller reference in the character
  (Default|SetPlayerControllerReference (Variables|Default|GetCharacterBP) self))

(event Input|EnhancedActionEvents|EnhancedInputActionIA_Journal
  (params (ActionValue :type Boolean) (ElapsedSeconds :type Float%20%28double-precision%29) (TriggeredSeconds :type Float%20%28double-precision%29) (InputAction :type Input%20Action%20Object%20Reference :default "/Game/Input/IA_Journal.IA_Journal"))
  ;[1 1 1] Oopen & Close Objective Journal
  (:Started
    (if (Variables|Default|GetJournalUnlocked)
      (if (Variables|Default|GetObjectiveJournalOnScreen)
        ;;[1 1 1] Journal Close Sound
        (Audio|PlaySound2D 0 1.0 1.0 0.0 0 0)
        (Widget|RemovefromParent (stale _returnvalue))
        (Variables|Default|SetObjectiveJournalOnScreen false)
        (else
          ;;[1 1 1] Journal Open Sound
          (Audio|PlaySound2D 0 1.0 1.0 0.0 0 0)
          (bind _returnvalue (UserInterface|CreateWidget "/Game/UI/Widgets/WB_ObjectiveJournalHUD.WB_ObjectiveJournalHUD_C" (Game|GetPlayerController 0)))
          (UserInterface|Viewport|AddtoViewport _returnvalue 0)
          (Variables|Default|SetObjectiveJournalOnScreen true)))
      (else
        (Development|PrintString "DEBUG | Journal Locked")
        ;;[1 1 1] Locked Journal Sound
        (Audio|PlaySound2D 0 1.0 1.0 0.0 0 0)))))

(event EventOnReferenceInitialized
  (params (ControlledPlayerCharacter :type Player%20Character%20Object%20Reference) (State :type %20Object%20Reference))
  ;[1 1 1] Initialization
  (CallFunction|SetBPReferences ControlledPlayerCharacter State)
  (CallFunction|SetControlleronCharacter)
  (CallFunction|ShowHUD))

(event Input|KeyboardEvents|T
  (params (Key :type Key%20Structure :default "None"))
  ;[1 1 1] Create Tutorial
  (:Pressed
    (bind _returnvalue (UserInterface|CreateWidget "/Game/UI/Widgets/WB_Tutorial.WB_Tutorial_C" (Game|GetPlayerController 0)))
    (UserInterface|Viewport|AddtoViewport _returnvalue 0)))

(fn ConstructionScript)