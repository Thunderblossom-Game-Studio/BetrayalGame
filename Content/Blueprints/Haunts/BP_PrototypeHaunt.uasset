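; BP_PrototypeHaunt is a prototype haunt that handles start, end and win outcomes for survivors versus a traitor.
; Ending the haunt triggers the traitor win unless the SurvivorWin flag was set by a survivor win.
; Each win shows its cutscene widget, starts a media sound and disables player 0's input for a fixed delay before restoring it.
; Debug strings print at each event.
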(event Custom|On%20Survivor%20Win
  (bind _returnvalue (Game|GetPlayerController 0))
  (Development|PrintString "SURVIVORS WIN")
  (Variables|Default|SetSurvivorWin true)
  (bind _returnvalue_2 (UserInterface|CreateWidget "/Game/Cutscenes/Sequencer_Movies/WB_HM_Player_Cutscene.WB_HM_Player_Cutscene_C"))
  (UserInterface|Viewport|AddtoViewport _returnvalue_2 0)
  (CameraShake|Start (Variables|Default|GetPlayerMediaSound))
  (Input|DisableInput _returnvalue)
  (Utilities|FlowControl|Delay 8.0)
  (Input|EnableInput _returnvalue))

(event Custom|On%20Traitor%20Win
  (bind _returnvalue (Game|GetPlayerController 0))
  (Development|PrintString "TRAITOR WIN")
  (bind _returnvalue_2 (UserInterface|CreateWidget "/Game/Cutscenes/Sequencer_Movies/WB_HM_Traitor_Cutscene.WB_HM_Traitor_Cutscene_C"))
  (UserInterface|Viewport|AddtoViewport _returnvalue_2 0)
  (CameraShake|Start (Variables|Default|GetTraitorMediaSound))
  (Input|DisableInput _returnvalue)
  (Utilities|FlowControl|Delay 9.0)
  (Input|EnableInput _returnvalue))

(event EventOnHauntStart
  (Development|PrintString "HAUNT STARTED"))

(event EventOnHauntEnd
  (Development|PrintString "HAUNT ENDED")
  (if (not (Variables|Default|GetSurvivorWin))
    (CallFunction|OnTraitorWin)))

(fn ConstructionScript)