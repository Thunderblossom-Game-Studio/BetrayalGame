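; Player character Blueprint that connects inventory, health, pause menu and push-to-talk voice chat to the player's UI.
; On begin play it caches BP_PlayerController when locally controlled, then forwards item pickup, removal, slot selection and damage events to it.
; Push-to-talk drives the voice chat subsystem and mic icon, while the pause input toggles WB_PauseMenu with input mode and cursor.
; A debug key calls ServerDropAllItems.
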(event Custom|On%20Slot%20Selected
  (params (Slot%20ID :type Inventory%20Slot%20Structure))
  ;[1 1 1] Update Highlighted Slot
  (Default|ItemEquiped (Variables|Default|GetPlayer%20Controller) Slot%20ID))

(event Custom|Set%20Player%20Controller
  ;[1 1 1] Set player controller reference
  (if (Pawn|IsLocallyControlled)
    (bind _asbp_player_controller (Utilities|Casting|CastToBP_PlayerController (Pawn|GetController)))
    (Variables|Default|SetPlayer%20Controller _asbp_player_controller)))

(event Custom|Update%20HUD
  (params (Slot :type Inventory%20Slot%20Structure))
  ;[1 1 1] Update Players Inventory
  (Default|UpdateInventory (Variables|Default|GetPlayer%20Controller) Slot))

(event Custom|Update%20Health%20UI
  ;[1 1 1] Take damage Update Health on Player HUD
  (Default|UpdatePlayerHealth (Variables|Default|GetPlayer%20Controller)))

(event Input|EnhancedActionEvents|EnhancedInputActionIA_PushToTalk
  (params (ActionValue :type Boolean) (ElapsedSeconds :type Float%20%28double-precision%29) (TriggeredSeconds :type Float%20%28double-precision%29) (InputAction :type Input%20Action%20Object%20Reference :default "/Game/Input/IA_PushToTalk.IA_PushToTalk"))
  (bind _returnvalue (Subsystems|GetVoiceChatSubsystem))
  ;[1 1 1] Push To Talk????
  (:Started
    (Class|VoiceChatSubsystem|StartPTT _returnvalue)
    (Default|UpdateMicIcon (Variables|Default|GetPlayer%20Controller) false true))
  (:Completed
    (Class|VoiceChatSubsystem|StopPTT _returnvalue)
    (Default|UpdateMicIcon (Variables|Default|GetPlayer%20Controller) false false)))

(event Input|EnhancedActionEvents|EnhancedInputActionIA_Pausemenu
  (params (ActionValue :type Boolean) (ElapsedSeconds :type Float%20%28double-precision%29) (TriggeredSeconds :type Float%20%28double-precision%29) (InputAction :type Input%20Action%20Object%20Reference :default "/Game/Input/IA_Pausemenu.IA_Pausemenu"))
  ;[1 1 1] Dispays Pausemenu and Tracks is activity.
  (:Started
    (CallFunction|DisplayPauseMenu)))

(event EventBeginPlay
  ;[1 1 1] Begin play
  (CallFunction|SetPlayerController))

(event EventOnItemPickedUp
  (params (Slot :type Inventory%20Slot%20Structure))
  ;[1 1 1] Update Players Inventory
  (CallFunction|UpdateHUD Slot))

(event EventOnItemRemovedfromInventory
  (params (Slot :type Inventory%20Slot%20Structure))
  ;[1 1 1] Update Players Inventory
  (CallFunction|UpdateHUD Slot))

(event EventOnSlotSelected
  (params (Slot :type Inventory%20Slot%20Structure))
  ;[1 1 1] Update Highlighted Slot
  (CallFunction|OnSlotSelected Slot))

(event EventOnDamageTaken
  (params (Damage :type Float%20%28single-precision%29))
  ;[1 1 1] Take damage Update Health on Player HUD
  (CallFunction|UpdateHealthUI))

(event Input|KeyboardEvents|DebugKeyH
  (params (Key :type Key%20Structure :default "None") (ActionValue :type Input%20Action%20Value%20Structure))
  (:Pressed
    (Class|PlayerCharacter|ServerDropAllItems)))

(event Input|KeyboardEvents|V
  (params (Key :type Key%20Structure :default "None"))
  ;[1 1 1] Debug health test  | Dsiabled Currently | Letter "V" Used By Push to talk system, Use new key
)

(fn ConstructionScript)

(fn DisplayPauseMenu
  (bind _returnvalue (Game|GetPlayerController 0))
  (if (Variables|Default|GetPauseMenuOnScreen)
    (Widget|RemovefromParent (stale _returnvalue_2))
    (Variables|Default|SetPauseMenuOnScreen false)
    (Input|SetInputModeGameOnly _returnvalue false)
    (Variables|/Script/Engine.PlayerController|SetbShowMouseCursor _returnvalue false)
    (else
      (bind _returnvalue_2 (UserInterface|CreateWidget "/Game/UI/Widgets/WB_PauseMenu.WB_PauseMenu_C" _returnvalue))
      (UserInterface|Viewport|AddtoViewport _returnvalue_2 0)
      (Input|SetInputModeUIOnly _returnvalue _returnvalue_2 "DoNotLock" false)
      (Variables|Default|SetPauseMenuOnScreen true)
      (Variables|/Script/Engine.PlayerController|SetbShowMouseCursor _returnvalue true))))