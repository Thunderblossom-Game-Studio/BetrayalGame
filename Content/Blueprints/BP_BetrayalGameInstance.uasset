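; Game instance for the Betrayal game that persists audio volume sliders and a tutorial-seen flag in the SavedSettings slot.
; On Init it loads that slot into a cached settings object, then initializes the menu player controller.
; A missing save triggers creation of a full-volume default save, which is written to disk but not cached.
; SaveSettings copies incoming values onto the cached object, rewriting the slot after each field.
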(event Custom|LoadSettings
  ;[0 0.3273 1] Load Settings
  (bind _returnvalue (SaveGame|LoadGamefromSlot (Variables|Default|GetSavedSettings)))
  (if (Utilities|IsValid _returnvalue)
    (bind _asbp_settings_save_object (Utilities|Casting|CastToBP_SettingsSaveObject _returnvalue))
    (Variables|Default|SetBP%20Settings%20Save%20Object _asbp_settings_save_object)
    (else
      ;;[1 1 1] If no save found load default settings
      (CallFunction|CreateSaveSlotObject))))

(event Custom|SaveSettings
  (params (Master%20VolumeSlider :type Float%20%28double-precision%29) (Ambient%20VolumeSlider :type Float%20%28double-precision%29) (Muisic%20Volume%20Slider :type Float%20%28double-precision%29) (SFX%20Volume%20Slider :type Float%20%28double-precision%29) (Ui%20Volume%20Slider :type Float%20%28double-precision%29) (Tutorial%20Seen? :type Boolean))
  (bind _bp_settings_save_object (Variables|Default|GetBP%20Settings%20Save%20Object))
  ;[1 1 1] Save Settings
  (Utilities|FlowControl|Sequence
    (:then_0
      (Variables|/Game/UI/BP_SettingsSaveObject.BP_SettingsSaveObject_C|SetMasterVolumeSlider _bp_settings_save_object Master%20VolumeSlider))
    (:then_1
      (Variables|/Game/UI/BP_SettingsSaveObject.BP_SettingsSaveObject_C|SetAmbientVolumeSlider _bp_settings_save_object Ambient%20VolumeSlider))
    (:then_2
      (Variables|/Game/UI/BP_SettingsSaveObject.BP_SettingsSaveObject_C|SetMusicVolumeSlider _bp_settings_save_object Muisic%20Volume%20Slider))
    (:then_3
      (Variables|/Game/UI/BP_SettingsSaveObject.BP_SettingsSaveObject_C|SetSFXVolumeSlider _bp_settings_save_object SFX%20Volume%20Slider))
    (:then_4
      (Variables|/Game/UI/BP_SettingsSaveObject.BP_SettingsSaveObject_C|SetUIVolumeSlider _bp_settings_save_object Ui%20Volume%20Slider))
    (:then_5
      (Variables|/Game/UI/BP_SettingsSaveObject.BP_SettingsSaveObject_C|SetTutorial%20Seen? _bp_settings_save_object Tutorial%20Seen?)))
  (SaveGame|SaveGametoSlot (Variables|Default|GetBP%20Settings%20Save%20Object) (Variables|Default|GetSavedSettings)))

(event EventInit
  ;[1 1 1] Once Initialized Load Settings | To create the Original Save object
  (CallFunction|LoadSettings)
  ;[1 1 1] Handle controller init
  (bind _asmenu_player_controller (Utilities|Casting|CastToMenu_PlayerController (Game|GetPlayerController 0)))
  (Class|MenuPlayerController|Init _asmenu_player_controller))

(fn CreateSaveSlotObject
  ;[1 1 1] Create Save Slot
  (bind _returnvalue (SaveGame|CreateSaveGameObject "/Game/UI/BP_SettingsSaveObject.BP_SettingsSaveObject_C"))
  (Utilities|FlowControl|Sequence
    (:then_0
      (Variables|/Game/UI/BP_SettingsSaveObject.BP_SettingsSaveObject_C|SetMasterVolumeSlider _returnvalue 1.0))
    (:then_1
      (Variables|/Game/UI/BP_SettingsSaveObject.BP_SettingsSaveObject_C|SetAmbientVolumeSlider _returnvalue 1.0))
    (:then_2
      (Variables|/Game/UI/BP_SettingsSaveObject.BP_SettingsSaveObject_C|SetMusicVolumeSlider _returnvalue 1.0))
    (:then_3
      (Variables|/Game/UI/BP_SettingsSaveObject.BP_SettingsSaveObject_C|SetSFXVolumeSlider _returnvalue 1.0))
    (:then_4
      (Variables|/Game/UI/BP_SettingsSaveObject.BP_SettingsSaveObject_C|SetUIVolumeSlider _returnvalue 1.0)))
  (SaveGame|SaveGametoSlot _returnvalue (Variables|Default|GetSavedSettings)))