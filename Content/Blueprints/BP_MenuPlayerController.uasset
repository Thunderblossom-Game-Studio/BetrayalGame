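; Menu player controller that owns and switches the main menu, server browser, lobby room and password screens.
; InitController creates all four widgets hidden up front, then sets UI-only input with a visible cursor.
; Show and hide events call functions that toggle widget visibility, focusing on show; only ShowMainMenu checks widget validity.
; A helper event adds username widgets with ready state to the lobby member list.
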(event Custom|Init%20Controller
  (Utilities|FlowControl|Sequence
    (:then_0
      (Class|MenuPlayerController|Init))
    (:then_1
      ;[1 1 1] Create UI
      (bind _returnvalue (UserInterface|CreateWidget "/Game/UI/Widgets/WB_MainMenu.WB_MainMenu_C"))
      (bind _output_get (Variables|Default|SetWB_MainMenu _returnvalue))
      (UserInterface|Viewport|AddtoViewport _output_get 0)
      (Variables|/Script/UMG.Widget|SetVisibility _output_get "Hidden"))
    (:then_2
      (bind _returnvalue_2 (UserInterface|CreateWidget "/Game/UI/Widgets/WB_LobbyMenu.WB_LobbyMenu_C"))
      (bind _output_get_2 (Variables|Default|SetWB_Lobby _returnvalue_2))
      (UserInterface|Viewport|AddtoViewport _output_get_2 0)
      (Variables|/Script/UMG.Widget|SetVisibility _output_get_2 "Hidden"))
    (:then_3
      (bind _returnvalue_3 (UserInterface|CreateWidget "/Game/UI/Widgets/WB_LobbyRoom.WB_LobbyRoom_C"))
      (bind _output_get_3 (Variables|Default|SetWB_LobbyRoom _returnvalue_3))
      (UserInterface|Viewport|AddtoViewport _output_get_3 0)
      (Variables|/Script/UMG.Widget|SetVisibility _output_get_3 "Hidden"))
    (:then_4
      (bind _returnvalue_4 (UserInterface|CreateWidget "/Game/UI/Widgets/WB_Password.WB_Password_C"))
      (bind _output_get_4 (Variables|Default|SetWB_PasswordField _returnvalue_4))
      (UserInterface|Viewport|AddtoViewport _output_get_4 0)
      (Variables|/Script/UMG.Widget|SetVisibility _output_get_4 "Hidden"))
    (:then_5
      ;[1 1 1] Set Input
      (Input|SetInputModeUIOnly (Game|GetPlayerController 0) (Variables|Default|GetWB_MainMenu) "DoNotLock" false)
      (Variables|Default|SetbShowMouseCursor true))))

(event EventHideMainMenu
  ;[1 1 1] Hide Main Menu
  (CallFunction|HideMainMenu))

(event EventCreatePlayerNameTextWidget
  (params (PlayerName :type String) (bIsReady :type Boolean) (ParentWidget :type Panel%20Widget%20Object%20Reference))
  ;[1 1 1] Handles Username Widget for Lobby Member List
  (bind _returnvalue (UserInterface|CreateWidget "/Game/UI/Widgets/WB_Username.WB_Username_C" self))
  (Default|SetName _returnvalue PlayerName bIsReady)
  (Widget|Panel|AddChild ParentWidget _returnvalue))

(event EventShowLobby
  ;[1 1 1] Show Server Browser
  (CallFunction|ShowServerBrowser))

(event EventHideLobby
  ;[1 1 1] Hide Server Browser
  (CallFunction|HideServerBrowser))

(event EventShowPasswordField
  ;[1 1 1] Show Password
  (CallFunction|ShowPasswordField))

(event EventHidePasswordField
  ;[1 1 1] Hide Password
  (CallFunction|HidePasswordField))

(event EventShowLobbyRoom
  ;[1 1 1] Show Lobby Room
  (CallFunction|ShowLobbyRoom))

(event EventHideLobbyRoom
  ;[1 1 1] Hide Lobby Room
  (CallFunction|HideLobbyRoom))

(event EventShowMainMenu
  ;[1 1 1] Show Main Menu
  (CallFunction|ShowMainMenu))

(fn ConstructionScript)

(fn ShowServerBrowser
  (bind _wb_lobby (Variables|Default|GetWB_Lobby))
  (Variables|/Script/UMG.Widget|SetVisibility _wb_lobby "Visible")
  (Widget|SetFocus _wb_lobby))

(fn HideServerBrowser
  (Widget|SetVisibility (Variables|Default|GetWB_Lobby) "Hidden"))

(fn ShowPasswordField
  (bind _wb_passwordfield (Variables|Default|GetWB_PasswordField))
  (Variables|/Script/UMG.Widget|SetVisibility _wb_passwordfield "Visible")
  (Widget|SetFocus _wb_passwordfield))

(fn HidePasswordField
  (Variables|/Script/UMG.Widget|SetVisibility (Variables|Default|GetWB_PasswordField) "Hidden"))

(fn ShowLobbyRoom
  (bind _wb_lobbyroom (Variables|Default|GetWB_LobbyRoom))
  (Variables|/Script/UMG.Widget|SetVisibility _wb_lobbyroom "Visible")
  (Widget|SetFocus _wb_lobbyroom))

(fn HideLobbyRoom
  (Variables|/Script/UMG.Widget|SetVisibility (Variables|Default|GetWB_LobbyRoom) "Hidden"))

(fn ShowMainMenu
  (bind _wb_mainmenu (Variables|Default|GetWB_MainMenu))
  (if (Utilities|IsValid _wb_mainmenu)
    (Variables|/Script/UMG.Widget|SetVisibility _wb_mainmenu "Visible")
    (Widget|SetFocus _wb_mainmenu)
    (else
      (Development|PrintString "ShowMainMenu Error: WB_MainMenu not valid!" true true "(R=0.937000,G=0.000000,B=0.000000,A=1.000000)"))))

(fn HideMainMenu
  (Variables|/Script/UMG.Widget|SetVisibility (Variables|Default|GetWB_MainMenu) "Hidden"))