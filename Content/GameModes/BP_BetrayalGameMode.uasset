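; BP_BetrayalGameMode is the game mode that shows intro widgets when game stages begin.
; The preparing stage waits briefly, then plays the WB_GameStart animation; the haunting stage plays WB_HauntStart immediately.
; Each widget is created for player controller 0 only and removed after a hard-coded delay rather than on animation completion.
; The exploring and finishing stage events are empty.
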(event EventBeginPlay)

(event EventTick
  (params (DeltaSeconds :type Float%20%28single-precision%29)))

(event EventOnExploringStageStart
  ;[1 1 1] Custom Game Stage Events
)

(event EventOnPreparingStageStart
  ;[1 1 1] Custom Game Stage Events
  ;[1 1 1] Game Start Widget
  (Utilities|FlowControl|Delay 1.0)
  (bind _asplayer_controller (Utilities|Casting|CastToPlayerController (Game|GetPlayerController 0)))
  (bind _returnvalue (UserInterface|CreateWidget "/Game/UI/WB_GameStart.WB_GameStart_C" _asplayer_controller))
  (UserInterface|Viewport|AddtoViewport _returnvalue 0)
  (UserInterface|Animation|PlayAnimation _returnvalue (Variables|/Game/UI/WB_GameStart.WB_GameStart_C|GetUI_ANI_GameStart _returnvalue) 0.0 1 "Forward" 1.0 false)
  (Utilities|FlowControl|Delay 4.1)
  (Widget|RemovefromParent _returnvalue))

(event EventOnHauntingStageStart
  ;[1 1 1] Custom Game Stage Events
  ;[1 1 1] Haunt Start Widget
  (bind _asplayer_controller (Utilities|Casting|CastToPlayerController (Game|GetPlayerController 0)))
  (bind _returnvalue (UserInterface|CreateWidget "/Game/UI/WB_HauntStart.WB_HauntStart_C" _asplayer_controller))
  (UserInterface|Viewport|AddtoViewport _returnvalue 0)
  (UserInterface|Animation|PlayAnimation _returnvalue (Variables|/Game/UI/WB_HauntStart.WB_HauntStart_C|GetUI_ANI_HauntStart_1 _returnvalue) 0.0 1 "Forward" 1.0 false)
  (Utilities|FlowControl|Delay 8.0)
  (Widget|RemovefromParent _returnvalue))

(event EventOnFinishingStageStart
  ;[1 1 1] Custom Game Stage Events
)

(fn ConstructionScript)