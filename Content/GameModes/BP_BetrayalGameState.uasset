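; BP_BetrayalGameState is a game state Blueprint that reacts to Lobby, Exploring, Haunting and Finishing stage start events.
; Exploring and Haunting show timed intro widgets (WB_GameStart, WB_HauntStart) on player controller 0, play their animations, then remove them.
; The Lobby handler is empty, and the Finishing handler only casts the controlled pawn to BP_PlayerCharacter without further action.
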(event EventBeginPlay)

(event EventTick
  (params (DeltaSeconds :type Float%20%28single-precision%29)))

(event EventOnHauntingStageStart
  ;[1 1 1] Stage Events
  ;[1 1 1] Comment
  (bind _returnvalue (UserInterface|CreateWidget "/Game/UI/WB_HauntStart.WB_HauntStart_C" (Game|GetPlayerController 0)))
  (UserInterface|Viewport|AddtoViewport _returnvalue 0)
  (UserInterface|Animation|PlayAnimation _returnvalue (Variables|/Game/UI/WB_HauntStart.WB_HauntStart_C|GetUI_ANI_HauntStart_1 _returnvalue) 0.0 1 "Forward" 1.0 false)
  (Utilities|FlowControl|Delay 8.0)
  (Widget|RemovefromParent _returnvalue))

(event EventOnFinishingStageStart
  ;[1 1 1] Stage Events
  (Utilities|Casting|CastToBP_PlayerCharacter (Pawn|GetControlledPawn (Game|GetPlayerController 0))))

(event EventOnLobbyStageStart
  ;[1 1 1] Stage Events
)

(event EventOnExploringStageStart
  ;[1 1 1] Stage Events
  ;[1 1 1] Start Widget
  (Utilities|FlowControl|Delay 1.0)
  (bind _returnvalue (UserInterface|CreateWidget "/Game/UI/WB_GameStart.WB_GameStart_C" (Game|GetPlayerController 0)))
  (UserInterface|Viewport|AddtoViewport _returnvalue 0)
  (UserInterface|Animation|PlayAnimation _returnvalue (Variables|/Game/UI/WB_GameStart.WB_GameStart_C|GetUI_ANI_GameStart _returnvalue) 0.0 1 "Forward" 1.0 false)
  (Utilities|FlowControl|Delay 4.1)
  (Widget|RemovefromParent _returnvalue))

(fn ConstructionScript)